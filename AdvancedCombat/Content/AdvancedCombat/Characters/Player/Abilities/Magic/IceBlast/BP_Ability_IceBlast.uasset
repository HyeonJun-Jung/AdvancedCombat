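; Gameplay Ability that fires an ice blast spell from the player's staff.
; On activation it commits, casts the avatar to Character and spawns BP_IceBlast at the mesh's staff_shoot socket, aimed along the control rotation with the character as instigator.
; It then ends immediately, leaving any further behavior to the spawned actor.
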(event Ability|EventActivateAbility
  (Ability|CommitAbility)
  (bind _as캐릭터 (Utilities|Casting|CastToCharacter (Ability|GetAvatarActorfromActorInfo)))
  (Game|SpawnActorfromClass "/Game/AdvancedCombat/Characters/Player/Abilities/Magic/IceBlast/BP_IceBlast.BP_IceBlast_C" (Math|Transform|MakeTransform (Transformation|GetSocketLocation (Variables|/Script/Engine.Character|GetMesh _as캐릭터) "staff_shoot") (Pawn|GetControlRotation _as캐릭터 :!class /Script/Engine.Pawn)) "Undefined" "MultiplyWithRoot" 0 _as캐릭터)
  (Ability|EndAbility))

(event Ability|EventOnEndAbility
  (params (bWasCancelled :type Boolean)))