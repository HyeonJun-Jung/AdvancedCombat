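; Gameplay ability for the player's katana combo attack, playing the katana attack montage once committed.
; It sets the max combo on the player's EquipComponent and loops on input presses, flagging the next attack while attack input is allowed.
; The ability ends on montage completion, failed setup, or a montage-ended callback, except interruptions of the GreatSword montage, which the check references instead of the katana one.
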(event Custom|OnMontageEnded_Event
  (params (Montage :type Anim%20Montage%20Object%20Reference) (bInterrupted :type Boolean))
  (if (or (and (!= Montage "/Game/AdvancedCombat/Characters/Player/Animation/GreatSword/Montage/AM_GreatSword_Attack.AM_GreatSword_Attack") bInterrupted) (not bInterrupted))
    (Ability|EndAbility)))

(event Ability|EventActivateAbility
  (bind _returnvalue (Game|Player|GetPlayerPawn 0))
  (bind _returnvalue_2 (Actor|GetComponentbyClass _returnvalue "/Script/AdvancedCombat.EquipComponent"))
  (bind _returnvalue_3 (Ability|CommitAbility))
  (Utilities|IsValid _returnvalue_2
    (:Is%20Valid
      (bind _output_get (Variables|Default|SetEquipComponent _returnvalue_2))
      (Variables|/Script/AdvancedCombat.EquipComponent|SetMaxCombo _output_get 4)
      (EventDispatchers|AssignOnMontageEnded (Components|SkeletalMesh|GetAnimInstance (Variables|/Script/Engine.Character|GetMesh (Game|GetPlayerCharacter 0))) (delegate Custom|OnMontageEnded_Event))
      (if _returnvalue_3
        (|PlayMontageandWaitProxy "None" "/Game/AdvancedCombat/Characters/Player/Animation/Katana_Knight/Montage/AM_Knight_Katana_Attack.AM_Knight_Katana_Attack" 1.0 "None" true 1.0 0.0 false
          (:then
            (Ability|Tasks|WaitInputPress false :!label _label
              (:OnPress
                (if (Variables|/Script/AdvancedCombat.EquipComponent|GetbCanAttackInput (Variables|Default|GetEquipComponent))
                  (Variables|/Script/AdvancedCombat.EquipComponent|SetbShouldDoNextAttack (Variables|Default|GetEquipComponent) true)
                  (goto _label)
                  (else
                    (goto _label))))))
          (:OnCompleted
            _))))
    (:Is%20Not%20Valid
      _))
  (Ability|EndAbility))

(event Ability|EventOnEndAbility
  (params (bWasCancelled :type Boolean)))

(fn GetNextComboSection
  (params (Current%20Combo :type Integer))
  (return (Utilities|String|StringToName (Utilities|String|ToString(Integer) (+ Current%20Combo 1)))))