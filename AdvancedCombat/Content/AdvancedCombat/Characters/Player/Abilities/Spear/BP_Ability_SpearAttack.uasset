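; Gameplay ability that runs the player's spear attack combo, capped at three hits through the avatar's EquipComponent.
; After committing, it plays the spear attack montage and repeatedly waits for input presses, flagging the next attack on EquipComponent whenever attack input is allowed.
; An AnimInstance montage-ended binding ends the ability, except when the spear montage itself is interrupted.
; Missing character, component or anim instance, or a failed commit, ends it immediately.
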(event Custom|OnMontageEnded_Event
  (params (Montage :type Anim%20Montage%20Object%20Reference) (bInterrupted :type Boolean))
  (if (or (and (!= Montage "/Game/AdvancedCombat/Characters/Player/Animation/Spear/Montage/AM_Spear_Attack.AM_Spear_Attack") bInterrupted) (not bInterrupted))
    (Ability|EndAbility)))

(event Ability|EventActivateAbility
  (bind _as캐릭터 (Utilities|Casting|CastToCharacter (Ability|GetAvatarActorfromActorInfo))
    (:then
      (Utilities|IsValid (Actor|GetComponentbyClass _as캐릭터 "/Script/AdvancedCombat.EquipComponent")
        (:Is%20Valid
          (bind _output_get (Variables|Default|SetEquipComp (Actor|GetComponentbyClass _as캐릭터 "/Script/AdvancedCombat.EquipComponent")))
          (Variables|/Script/AdvancedCombat.EquipComponent|SetMaxCombo _output_get 3)
          (bind _ascombat_player_anim_instance (Utilities|Casting|CastToCombatPlayer_AnimInstance (Components|SkeletalMesh|GetAnimInstance (Variables|/Script/Engine.Character|GetMesh _as캐릭터)))
            (:then
              (Variables|Default|SetAs%20Combat%20Player%20Anim%20Instance _ascombat_player_anim_instance)
              (EventDispatchers|AssignOnMontageEnded (Components|SkeletalMesh|GetAnimInstance (Variables|/Script/Engine.Character|GetMesh _as캐릭터)) (delegate Custom|OnMontageEnded_Event))
              (bind _returnvalue (Ability|CommitAbility))
              (if _returnvalue
                (|PlayMontageandWaitProxy "None" "/Game/AdvancedCombat/Characters/Player/Animation/Spear/Montage/AM_Spear_Attack.AM_Spear_Attack" 1.0 "None" true 1.0 0.0 false
                  (:then
                    (Ability|Tasks|WaitInputPress false :!label _label
                      (:OnPress
                        (if (Variables|/Script/AdvancedCombat.EquipComponent|GetbCanAttackInput (Variables|Default|GetEquipComp))
                          (Variables|/Script/AdvancedCombat.EquipComponent|SetbShouldDoNextAttack (Variables|Default|GetEquipComp) true)
                          (goto _label)
                          (else
                            (goto _label)))))))
                (else
                  _)))
            (:CastFailed
              _)))
        (:Is%20Not%20Valid
          _)))
    (:CastFailed
      _))
  (Ability|EndAbility))

(event Ability|EventOnEndAbility
  (params (bWasCancelled :type Boolean)))