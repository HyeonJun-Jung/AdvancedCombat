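; Greatsword defense Gameplay Ability that holds the player character in a guard while the input is held.
; Activation commits the ability and sets the anim instance's Defensing flag; input release clears it, removes the loose Parryable state tag and ends the ability.
; Guard and parry reaction events play Katana montages, with guard hits choosing left or right by hit direction and frontal hits picking one at random.
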(event Custom|Show%20Guard%20Reaction
  (params (hitDirection :type EACHitReactDirection%20Enum :default "None"))
  (switch Utilities|FlowControl|Switch|SwitchonEACHitReactDirection hitDirection
    (:Left
      (|PlayMontageandWaitProxy "None" "/Game/AdvancedCombat/Characters/Player/Animation/Katana_Knight/Montage/AM_Knight_Katana_GuardSucces_L.AM_Knight_Katana_GuardSucces_L" 1.0 "None" true 1.0 0.0 false :!label _label))
    (:Front
      (switch int (Math|Random|RandomIntegerinRange 0 1)
        (:0
          (goto _label))
        (:1
          (|PlayMontageandWaitProxy "None" "/Game/AdvancedCombat/Characters/Player/Animation/Katana_Knight/Montage/AM_Knight_Katana_GuardSucces_R.AM_Knight_Katana_GuardSucces_R" 1.0 "None" true 1.0 0.0 false :!label _label_2))))
    (:Right
      (goto _label_2))))

(event Custom|Show%20Parry%20Reaction
  (params (hitDirection :type EACHitReactDirection%20Enum :default "None"))
  (|PlayMontageandWaitProxy "None" "/Game/AdvancedCombat/Characters/Player/Animation/Katana_Knight/Montage/AM_Knight_Katana_Parry.AM_Knight_Katana_Parry" 1.0 "None" true 1.0 0.0 false))

(event Ability|EventActivateAbility
  (bind _ascharacter_base (Utilities|Casting|CastToCharacter_Base (Ability|GetAvatarActorfromActorInfo))
    (:then
      (bind _ascombat_player_anim_instance (Utilities|Casting|CastToCombatPlayer_AnimInstance (Components|SkeletalMesh|GetAnimInstance (Variables|/Script/Engine.Character|GetMesh _ascharacter_base)))
        (:then
          (Variables|Default|SetAs%20Combat%20Player%20Anim%20Instance _ascombat_player_anim_instance)
          (bind _returnvalue (Ability|CommitAbility))
          (if _returnvalue
            (Variables|/Script/AdvancedCombat.CombatPlayer_AnimInstance|SetbDefensing _ascombat_player_anim_instance true)
            (Ability|Tasks|WaitInputRelease false
              (:OnRelease
                (Variables|/Script/AdvancedCombat.CombatPlayer_AnimInstance|SetbDefensing (Variables|Default|GetAs%20Combat%20Player%20Anim%20Instance) false)
                (Ability|GameplayEffect|RemoveLooseGameplayTags (Ability|GetAvatarActorfromActorInfo) (GameplayTags|MakeGameplayTagContainerfromTag (GameplayTags|MakeLiteralGameplayTag "(TagName=\"Character.State.Parryable\")")))))))
        (:CastFailed
          _)))
    (:CastFailed
      _))
  (Ability|EndAbility))

(event Ability|EventOnEndAbility
  (params (bWasCancelled :type Boolean)))