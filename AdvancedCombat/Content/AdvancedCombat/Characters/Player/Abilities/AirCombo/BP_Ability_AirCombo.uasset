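; Gameplay ability that plays the player's air combo montage, holding the character airborne in Flying movement mode.
; It sets the EquipComponent's combo limit, then repeatedly waits for input presses, flagging the next attack whenever attack input is allowed.
; Montage completion, failed setup, or any montage-ended event except an interruption of the combo montage itself restores the saved movement mode and ends the ability.
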(event Custom|OnMontageEnded_Event
  (params (Montage :type Anim%20Montage%20Object%20Reference) (bInterrupted :type Boolean))
  (if (or (and (!= Montage "/Game/AdvancedCombat/Characters/Player/Animation/AirCombo/AM_AirCombo.AM_AirCombo") bInterrupted) (not bInterrupted))
    (bind _as캐릭터 (Utilities|Casting|CastToCharacter (Ability|GetAvatarActorfromActorInfo)))
    (Pawn|Components|CharacterMovement|SetMovementMode (Variables|/Script/Engine.Character|GetCharacterMovement _as캐릭터) (Variables|Default|GetLocal%20Movement%20Mode) 0)
    (Ability|EndAbility)))

(event Ability|EventActivateAbility
  (bind _returnvalue (Game|Player|GetPlayerPawn 0))
  (bind _returnvalue_2 (Actor|GetComponentbyClass _returnvalue "/Script/AdvancedCombat.EquipComponent"))
  (bind _returnvalue_3 (Ability|CommitAbility))
  (Utilities|IsValid _returnvalue_2
    (:Is%20Valid
      (bind _output_get (Variables|Default|SetEquipComponent _returnvalue_2))
      (Variables|/Script/AdvancedCombat.EquipComponent|SetMaxCombo _output_get 4)
      (EventDispatchers|AssignOnMontageEnded (Components|SkeletalMesh|GetAnimInstance (Variables|/Script/Engine.Character|GetMesh (Game|GetPlayerCharacter 0))) (delegate Custom|OnMontageEnded_Event))
      (if _returnvalue_3
        (bind _as캐릭터 (Utilities|Casting|CastToCharacter (Ability|GetAvatarActorfromActorInfo))
          (:then
            (Variables|Default|SetLocal%20Movement%20Mode (Variables|/Script/Engine.CharacterMovementComponent|GetMovementMode (Variables|/Script/Engine.Character|GetCharacterMovement _as캐릭터)))
            (Pawn|Components|CharacterMovement|SetMovementMode (Variables|/Script/Engine.Character|GetCharacterMovement _as캐릭터) "MOVE_Flying" 0)
            (|PlayMontageandWaitProxy "None" "/Game/AdvancedCombat/Characters/Player/Animation/AirCombo/AM_AirCombo.AM_AirCombo" 1.0 "None" true 1.0 0.0 false
              (:then
                (Ability|Tasks|WaitInputPress false :!label _label
                  (:OnPress
                    (if (Variables|/Script/AdvancedCombat.EquipComponent|GetbCanAttackInput (Variables|Default|GetEquipComponent))
                      (Variables|/Script/AdvancedCombat.EquipComponent|SetbShouldDoNextAttack (Variables|Default|GetEquipComponent) true)
                      (goto _label)
                      (else
                        (goto _label))))))
              (:OnCompleted
                _)))
          (:CastFailed
            _))))
    (:Is%20Not%20Valid
      _))
  (bind _as캐릭터_2 (Utilities|Casting|CastToCharacter (Ability|GetAvatarActorfromActorInfo)))
  (Pawn|Components|CharacterMovement|SetMovementMode (Variables|/Script/Engine.Character|GetCharacterMovement _as캐릭터_2) (Variables|Default|GetLocal%20Movement%20Mode) 0)
  (Ability|EndAbility))

(event Ability|EventOnEndAbility
  (params (bWasCancelled :type Boolean)))