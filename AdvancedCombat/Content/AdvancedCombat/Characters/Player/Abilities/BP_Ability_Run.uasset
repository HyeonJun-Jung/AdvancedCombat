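; Gameplay ability that lets the player character run while the ability input is held.
; On activation it commits, caches the avatar's max walk speed and raises it by 40%.
; Input release restores the cached speed, removes owner effects tagged Character.Ability.Run and ends the ability.
; A failed commit or cast skips straight to that removal and end, and OnEndAbility does nothing.
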(event Ability|EventActivateAbility
  (bind _returnvalue (Ability|CommitAbility))
  (if _returnvalue
    (bind _as캐릭터 (Utilities|Casting|CastToCharacter (Ability|GetAvatarActorfromActorInfo))
      (:then
        (bind _output_get (Variables|Default|SetLocal%20Max%20Walk%20Speed (Variables|/Script/Engine.CharacterMovementComponent|GetMaxWalkSpeed (Variables|/Script/Engine.Character|GetCharacterMovement _as캐릭터))))
        (Variables|/Script/Engine.CharacterMovementComponent|SetMaxWalkSpeed (Variables|/Script/Engine.Character|GetCharacterMovement _as캐릭터) (* _output_get 1.4))
        (Ability|Tasks|WaitInputRelease false
          (:OnRelease
            (Variables|/Script/Engine.CharacterMovementComponent|SetMaxWalkSpeed (Variables|/Script/Engine.Character|GetCharacterMovement _as캐릭터) (Variables|Default|GetLocal%20Max%20Walk%20Speed)))))
      (:CastFailed
        _)))
  (Ability|RemoveGameplayEffectFromOwnerWithAssetTags "(GameplayTags=((TagName=\"Character.Ability.Run\")))")
  (Ability|EndAbility))

(event Ability|EventOnEndAbility
  (params (bWasCancelled :type Boolean)))