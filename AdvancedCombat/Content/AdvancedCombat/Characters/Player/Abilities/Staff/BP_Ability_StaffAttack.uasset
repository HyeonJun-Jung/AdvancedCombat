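; Gameplay ability for the player's staff attack, managing a combo capped at three hits through the EquipComponent.
; On activation it hooks the CombatPlayer anim instance's attack-end delegate, commits, then flags the first attack.
; A re-arming WaitInputPress loop flags the next attack whenever a press arrives while attack input is allowed.
; Attack end, failed commit or failed anim-instance cast clears both combo flags and ends the ability.
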(event Custom|OnMontageEnded_Event
  (params (Montage :type Anim%20Montage%20Object%20Reference) (bInterrupted :type Boolean))
  (bind _equipcomp (Variables|Default|GetEquipComp))
  (Variables|/Script/AdvancedCombat.EquipComponent|SetbCanAttackInput _equipcomp false)
  (Variables|/Script/AdvancedCombat.EquipComponent|SetbShouldDoNextAttack _equipcomp false)
  (Ability|EndAbility))

(event Custom|Delegate_AttackEnd_Event
  (bind _equipcomp (Variables|Default|GetEquipComp))
  (Variables|/Script/AdvancedCombat.EquipComponent|SetbCanAttackInput _equipcomp false)
  (Variables|/Script/AdvancedCombat.EquipComponent|SetbShouldDoNextAttack _equipcomp false)
  (Ability|EndAbility))

(event Ability|EventActivateAbility
  (bind _as캐릭터 (Utilities|Casting|CastToCharacter (Ability|GetAvatarActorfromActorInfo)))
  (Utilities|IsValid (Actor|GetComponentbyClass _as캐릭터 "/Script/AdvancedCombat.EquipComponent")
    (:Is%20Valid
      (bind _output_get (Variables|Default|SetEquipComp (Actor|GetComponentbyClass _as캐릭터 "/Script/AdvancedCombat.EquipComponent")))
      (Variables|/Script/AdvancedCombat.EquipComponent|SetMaxCombo _output_get 3)
      (bind _ascombat_player_anim_instance (Utilities|Casting|CastToCombatPlayer_AnimInstance (Components|SkeletalMesh|GetAnimInstance (Variables|/Script/Engine.Character|GetMesh _as캐릭터)))
        (:then
          (bind _output_get_2 (Variables|Default|SetAs%20Combat%20Player%20Anim%20Instance _ascombat_player_anim_instance))
          (EventDispatchers|AssignDelegateAttackEnd _output_get_2 (delegate Custom|Delegate_AttackEnd_Event))
          (bind _returnvalue (Ability|CommitAbility))
          (if _returnvalue
            (Variables|/Script/AdvancedCombat.EquipComponent|SetbShouldDoNextAttack (Variables|Default|GetEquipComp) true)
            (Ability|Tasks|WaitInputPress false :!label _label
              (:OnPress
                (if (Variables|/Script/AdvancedCombat.EquipComponent|GetbCanAttackInput (Variables|Default|GetEquipComp))
                  (Variables|/Script/AdvancedCombat.EquipComponent|SetbShouldDoNextAttack (Variables|Default|GetEquipComp) true)
                  (goto _label)
                  (else
                    (goto _label)))))
            (else
              _)))
        (:CastFailed
          _))
      (Variables|/Script/AdvancedCombat.EquipComponent|SetbCanAttackInput (Variables|Default|GetEquipComp) false)
      (Variables|/Script/AdvancedCombat.EquipComponent|SetbShouldDoNextAttack (Variables|Default|GetEquipComp) false)
      (Ability|EndAbility))
    (:Is%20Not%20Valid)))

(event Ability|EventOnEndAbility
  (params (bWasCancelled :type Boolean)))