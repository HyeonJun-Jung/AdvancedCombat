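; Test character for the parkour system that delegates traversal to a TraversalComponent, initialized with its motion warping component and follow camera.
; Jump triggers traversal actions, C drops from a climb, and move events feed or reset the component's movement.
; V runs a vault test: it sets height, depth and vault warp targets from tagged reference cubes, then plays the montage in Flying mode without collision, restoring both on blend out.
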(event Input|EnhancedActionEvents|EnhancedInputActionIA_Jump
  (params (ActionValue :type Boolean) (ElapsedSeconds :type Float%20%28double-precision%29) (TriggeredSeconds :type Float%20%28double-precision%29) (InputAction :type Input%20Action%20Object%20Reference :default "/Game/ThirdPerson/Input/Actions/IA_Jump.IA_Jump"))
  (:Started
    (Default|TriggerTraversalAction (Variables|Default|GetTraversalComponent) true)))

(event EventBeginPlay
  (Default|InitializeReferences (Variables|Default|GetTraversalComponent) self (Variables|Default|GetMotionWarping) (Variables|Default|GetFollowCamera)))

(event Collision|EventActorBeginOverlap
  (params (OtherActor :type Actor%20Object%20Reference)))

(event EventTick
  (params (DeltaSeconds :type Float%20%28single-precision%29)))

(event EventTraversalMove
  (params (ActionValueX :type Float%20%28single-precision%29) (ActionValueY :type Float%20%28single-precision%29))
  (bind _traversalcomponent (Variables|Default|GetTraversalComponent))
  (Default|AddMovementInput _traversalcomponent ActionValueX false)
  (Default|AddMovementInput _traversalcomponent ActionValueY true))

(event EventTraversalMoveEnd
  (Default|ResetMovement (Variables|Default|GetTraversalComponent)))

(event Input|KeyboardEvents|C
  (params (Key :type Key%20Structure :default "None"))
  (:Pressed
    (Default|DropfromClimb (Variables|Default|GetTraversalComponent))))

(event Input|KeyboardEvents|V
  (params (Key :type Key%20Structure :default "None"))
  (:Pressed
    (Collision|SetCollisionEnabled (Variables|Default|GetCapsuleComponent) "NoCollision")
    (Pawn|Components|CharacterMovement|SetMovementMode (Variables|Character|GetCharacterMovement) "MOVE_Flying" 0)
    ;[1 1 1] Height Warp
    (bind _outactors (Actor|GetAllActorsOfClasswithTag "/Game/AdvancedCombat/Parkour/Actors/BP_ReferencedCube.BP_ReferencedCube_C" "HeightWarpRef"))
    (Class|MotionWarpingComponent|AddorUpdateWarpTargetfromLocationandRotation (Variables|Default|GetMotionWarping) "HeightWarp" (- (Transformation|GetActorLocation (Utilities|Array|Get(acopy) _outactors)) "0.000000,0.000000,60.000000") (Transformation|GetActorRotation (Utilities|Array|Get(acopy) _outactors)))
    ;[1 1 1] Depth Warp
    (bind _outactors_2 (Actor|GetAllActorsOfClasswithTag "/Game/AdvancedCombat/Parkour/Actors/BP_ReferencedCube.BP_ReferencedCube_C" "DepthWarpRef"))
    (Class|MotionWarpingComponent|AddorUpdateWarpTargetfromLocationandRotation (Variables|Default|GetMotionWarping) "DepthWarp" (- (Transformation|GetActorLocation (Utilities|Array|Get(acopy) _outactors_2)) "0.000000,0.000000,45.000000") (Transformation|GetActorRotation (Utilities|Array|Get(acopy) _outactors_2)))
    ;[1 1 1] Vault Warp
    (bind _outactors_3 (Actor|GetAllActorsOfClasswithTag "/Game/AdvancedCombat/Parkour/Actors/BP_ReferencedCube.BP_ReferencedCube_C" "VaultWarpRef"))
    (Class|MotionWarpingComponent|AddorUpdateWarpTargetfromLocationandRotation (Variables|Default|GetMotionWarping) "VaultWarp" (+ (Transformation|GetActorLocation (Utilities|Array|Get(acopy) _outactors_3)) "0.000000,0.000000,3.000000") (Transformation|GetActorRotation (Utilities|Array|Get(acopy) _outactors_3)))
    (Animation|Montage|PlayMontage (Variables|Character|GetMesh) "/Game/AdvancedCombat/Parkour/Animations/KnightAnimations/Montage/AM_Knight_Vault.AM_Knight_Vault"
      (:OnBlendOut
        (Collision|SetCollisionEnabled (Variables|Default|GetCapsuleComponent) "QueryAndPhysics")
        (Pawn|Components|CharacterMovement|SetMovementMode (Variables|Character|GetCharacterMovement) "MOVE_Walking" 0)))))

(fn ConstructionScript)