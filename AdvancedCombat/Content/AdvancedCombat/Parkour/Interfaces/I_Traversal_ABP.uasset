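; Blueprint interface for pushing parkour traversal data into an animation Blueprint.
; It declares setters for traversal state, action, climb style and climb direction.
; Further setters pass left and right hand climb locations and rotations, plus foot climb locations.
; The functions are declarations only, so the implementing class supplies the behavior.
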(fn SetTraversalState
  (params (NewTraversalState :type Gameplay%20Tag%20Structure))
  (return false))

(fn SetTraversalAction
  (params (NewTraversalAction :type Gameplay%20Tag%20Structure))
  (return false))

(fn SetClimbStyle
  (params (NewClimbStyle :type Gameplay%20Tag%20Structure))
  (return false))

(fn SetClimbDirection
  (params (NewClimbDirection :type Gameplay%20Tag%20Structure))
  (return false))

(fn SetLeftHandClimbLocation
  (params (NewLeftHandClimbLocation :type Vector))
  (return false))

(fn SetRightHandClimbLocation
  (params (NewRightHandLocation :type Vector))
  (return false))

(fn SetLeftHandClimbRotation
  (params (NewLeftHandClimbRotation :type Rotator))
  (return false))

(fn SetRightHandClimbRotation
  (params (NewRightHandClimbRotation :type Rotator))
  (return false))

(fn SetLeftFootClimbLocation
  (params (NewLeftFootClimbLocation :type Vector))
  (return false))

(fn SetRightFootClimbLocation
  (params (NewRightFootLocation :type Vector))
  (return false))