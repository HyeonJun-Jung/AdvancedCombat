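; BP_Slash2 is a Samurai enemy slash attack actor that deals parryable damage to characters overlapping its box.
; Each overlapping actor is recorded in DamagedActors so it is processed only once.
; Hit characters are launched opposite their own facing, not away from the slash, then receive point damage with the ParryableDamage type.
; The actor destroys itself when its Niagara effect finishes.
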(event OnComponentBeginOverlap(Box)
  (params (OverlappedComponent :type Primitive%20Component%20Object%20Reference) (OtherActor :type Actor%20Object%20Reference) (OtherComp :type Primitive%20Component%20Object%20Reference) (OtherBodyIndex :type Integer) (bFromSweep :type Boolean) (SweepResult :type Hit%20Result%20Structure%20%28by%20ref%29))
  (if (not (Utilities|Array|ContainsItem (Variables|Default|GetDamagedActors) OtherActor))
    (Utilities|Array|Add (Variables|Default|GetDamagedActors) OtherActor)
    (bind _as캐릭터 (Utilities|Casting|CastToCharacter OtherActor))
    (Character|LaunchCharacter _as캐릭터 (* (Transformation|GetActorForwardVector _as캐릭터) -4e+02) false false)
    (Game|Damage|ApplyPointDamage _as캐릭터 1e+01 (Transformation|GetActorLocation) (Variables|Default|GetHit%20Info) 0 self "/Script/AdvancedCombat.ParryableDamage")))

(event OnSystemFinished(Niagara)
  (params (PSystem :type Niagara%20Component%20Object%20Reference))
  (Actor|DestroyActor))

(event EventBeginPlay)

(event Collision|EventActorBeginOverlap
  (params (OtherActor :type Actor%20Object%20Reference)))

(event EventTick
  (params (DeltaSeconds :type Float%20%28single-precision%29)))

(fn ConstructionScript)